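; Generic base puzzle Blueprint that reports its solved and unsolved state to an assigned PuzzleCollection.
; PuzzleSolved and PuzzleUnsolved pass the puzzle itself to the collection, which treats it as one part of a larger whole.
; A missing collection is meant only for end puzzles: BeginPlay prints a warning, solving prints a failure message, and unsolving does nothing.
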(event `self.ReceiveBeginPlay`
  ;[1 1 1] If the puzzle doesn't have a Collection, warns the devs
  (if (== (`self.PuzzleCollection`) null)
    (`KismetSystemLibrary.PrintString` (`KismetStringLibrary.Concat_StrStr` "Puzzle " (`KismetSystemLibrary.GetObjectName` self) " has no Collection assigned !" " \nThis is coherent only if this is an end puzzle."))))

(event `PuzzleSolved`
  (bind _puzzlecollection (`self.PuzzleCollection`))
  (if (!= _puzzlecollection null)
    (`/Game/Blueprints/BP_GenericPawnPuzzleCollection.SinglePuzzleSovled` _puzzlecollection self)
    (else
      (`KismetSystemLibrary.PrintString` "Failed to solve single puzzle !"))))

(event `PuzzleUnsolved`
  (bind _puzzlecollection (`self.PuzzleCollection`))
  (if (!= _puzzlecollection null)
    (`/Game/Blueprints/BP_GenericPawnPuzzleCollection.SinglePuzzleUnsolved` _puzzlecollection self)))

(fn `UserConstructionScript`)