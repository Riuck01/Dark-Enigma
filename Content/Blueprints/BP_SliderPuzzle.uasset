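; Timing puzzle where a pointer slides back and forth across a background bar and must be stopped inside a target.
; Tick moves the pointer child actor along local X, reversing at bounds derived from the background's world scale.
; InteractionTriggered stops it and checks the offset against the target's scaled width: a miss resumes after a delay, a hit calls PuzzleSolved.
; A dynamic emissive material shows idle, failed or solved through color and strength lookups.
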(event `self.ReceiveBeginPlay`
  (`parent.ReceiveBeginPlay`)
  ;[1 1 1] Creates a DMI for Target (namely to change its color)
  (bind _returnvalue (`PrimitiveComponent.CreateDynamicMaterialInstance` (`self.Target`) 0 "/Game/LevelPrototyping/Materials/M_Emissive.M_Emissive" "DMI_SliderPuzzleTargetEmissive"))
  (set `self.TargetDMI` _returnvalue)
  ;[1 1 1] Setup the DMI for Target
  (`self.SetTargetDMI_EmissiveColor` (`BlueprintMapLibrary.Map_Find` (`self.TargetDMI_Colors`) "Idling"))
  (`self.SetTargetDMI_EmissiveStrength` (`BlueprintMapLibrary.Map_Find` (`self.TargetDMI_Strengths`) "Dim")))

(event `self.ReceiveTick`
  (params (DeltaSeconds :type "Float (single-precision)"))
  (bind _x (.x (`self.AccumulatedOffset`)))
  (bind _returnvalue (`KismetMathLibrary.MakeVector` (`self.DistToMoveThisFrame`)))
  (bind _returnvalue_2 (* (`self.SliderSpeed (cm/s)`) DeltaSeconds))
  (bind _returnvalue_3 (* (.x (`SceneComponent.K2_GetComponentScale` (`self.Background`))) 100.0 0.5))
  (if (`self.IsMoving`)
    ;[1 1 1] Test if the slider has reached either limits and should change direction
    (if (`self.IsSliderMovingPositiveX`)
      ;;[1 1 1] Checks if slider went too far (X+)
      (if (>= _x _returnvalue_3)
        (set `self.IsSliderMovingPositiveX` false))
      (else
        ;;[1 1 1] Checks if slider went too far (X-)
        (if (<= _x (* _returnvalue_3 -1.0))
          (set `self.IsSliderMovingPositiveX` true))))
    ;[1 1 1] Calculates the distance to move this frame
    (if (`self.IsSliderMovingPositiveX`)
      (set `self.DistToMoveThisFrame` _returnvalue_2)
      (else
        (set `self.DistToMoveThisFrame` (* _returnvalue_2 -1.0))))
    ;[1 1 1] Calculates the new position, updates the accumulated offset, and applies the movement
    (set `self.AccumulatedOffset` (+ _returnvalue (`self.AccumulatedOffset`)))
    (`self.K2_AddActorLocalOffset` (`ChildActorComponent.ChildActor` (`self.BP_SliderPointer`)) _returnvalue false false)))

(event `/Game/Blueprints/BPI_Interactable.InteractionTriggered`
  (bind _x (.x (`self.AccumulatedOffset`)))
  (bind _returnvalue (* (.x (`SceneComponent.K2_GetComponentScale` (`self.Target`))) 100.0 0.5))
  (if (`self.IsMoving`)
    (set `self.IsMoving` false) ; Stops the Pointer
    ;[1 1 1] Checks if slider went too far (X+)
    (if (>= _x _returnvalue)
      ;[1 1 1] Failure scenario (restarts the puzzle after some time)
      (`self.SetTargetDMI_EmissiveColor` (`BlueprintMapLibrary.Map_Find` (`self.TargetDMI_Colors`) "Failed") :!label _label)
      (`self.SetTargetDMI_EmissiveStrength` (`BlueprintMapLibrary.Map_Find` (`self.TargetDMI_Strengths`) "Bright"))
      (`KismetSystemLibrary.Delay` 1.0)
      (set `self.IsMoving` true)
      (`self.SetTargetDMI_EmissiveColor` (`BlueprintMapLibrary.Map_Find` (`self.TargetDMI_Colors`) "Idling"))
      (`self.SetTargetDMI_EmissiveStrength` (`BlueprintMapLibrary.Map_Find` (`self.TargetDMI_Strengths`) "Dim"))
      (else
        ;[1 1 1] Checks if slider went too far (X-)
        (if (<= _x (* _returnvalue -1.0))
          (goto _label)
          (else
            ;[1 1 1] Success scenario (solves the puzzle forever)
            (`self.SetTargetDMI_EmissiveColor` (`BlueprintMapLibrary.Map_Find` (`self.TargetDMI_Colors`) "Solved"))
            (`self.SetTargetDMI_EmissiveStrength` (`BlueprintMapLibrary.Map_Find` (`self.TargetDMI_Strengths`) "Dim"))
            (`KismetSystemLibrary.PrintString` "Solved ! Should warn manager with an event here")
            (`self.PuzzleSolved`)))))))

(fn `GetTargetDMI_EmissionStrenght`
  (returns (RESEmissionStrenght :type "Float (double-precision)"))
  (bind _returnvalue (`MaterialInstanceDynamic.K2_GetScalarParameterValue` (`self.TargetDMI`) "Emission Strenght"))
  (return _returnvalue))

(fn `GetTargetDMI_EmissiveColor`
  (returns (RESEmissiveColor :type "Color Structure"))
  (bind _returnvalue (`MaterialInstanceDynamic.K2_GetVectorParameterValue` (`self.TargetDMI`) "NoneEmissive Color"))
  (return (`KismetMathLibrary.Conv_LinearColorToColor` _returnvalue)))

(fn `SetTargetDMI_EmissiveColor`
  (params (ARGEmissiveColor :type "Color Structure"))
  (`MaterialInstanceDynamic.SetVectorParameterValue` (`self.TargetDMI`) "Emissive Color" (`KismetMathLibrary.Conv_ColorToLinearColor` ARGEmissiveColor)))

(fn `SetTargetDMI_EmissiveStrength`
  (params (ARGEmissionStrenght :type "Float (double-precision)"))
  (`MaterialInstanceDynamic.SetScalarParameterValue` (`self.TargetDMI`) "Emission Strenght" ARGEmissionStrenght))

(fn `UserConstructionScript`)