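; BP_BlockedLightPuzzle is a puzzle actor with a wood plank, presumably blocking its light, that is removed through play.
; On BeginPlay it runs the parent logic, then applies the LightColor variable to its point and spot lights.
; InteractionTriggered and AllPuzzlesSolved share one path that destroys the plank component, guarded by a validity check because both events can fire in succession.
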(event `self.ReceiveBeginPlay`
  (`parent.ReceiveBeginPlay`)
  (`self.ApplyLightsColor`))

(event `/Game/Blueprints/BPI_Interactable.InteractionTriggered`
  (bind _woodplank (`self.WoodPlank`))
  ;[1 1 1] Destroy the plank
  (if (`KismetSystemLibrary.IsValid` _woodplank) :!label _label
    (`ActorComponent.K2_DestroyComponent` _woodplank)))

(event `self.AllPuzzlesSolved`
  (goto _label))

(fn `ApplyLightsColor`
  (bind _returnvalue (`KismetMathLibrary.Conv_ColorToLinearColor` (`self.LightColor`)))
  (`LightComponent.SetLightColor` (`self.PointLight`) _returnvalue true)
  (`LightComponent.SetLightColor` (`self.SpotLight`) _returnvalue true))

(fn `UserConstructionScript`)