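; Pawn for the cage puzzle that lets the player slide a cylinder piece left and right.
; Chain inputs offset the interacted object's MovingPiece by MoveVector while its world X is within the Placement1 and Placement4 markers.
; ResolveCollider overlaps call PuzzleSolved on begin and PuzzleUnsolved on end, printing debug text.
; The interact input hands possession back to the first-person character.
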(event `self.ReceiveBeginPlay`
  (set `self.ObjectInteracting` (`self.ObjectInteracting`))
  (set `self.LimitMove` (`self.LimitMove`)))

(event `self.ReceiveActorBeginOverlap`
  (params (OtherActor :type "Actor Object Reference")))

(event `EnhancedInput|/Game/FirstPerson/Input/Actions/IA_Interact`
  (params (ActionValue :type Boolean) (ElapsedSeconds :type "Float (double-precision)") (TriggeredSeconds :type "Float (double-precision)") (InputAction :type "InputAction Object Reference" :default "/Game/FirstPerson/Input/Actions/IA_Interact.IA_Interact"))
  ;[1 1 1] Back to Player
  (:`Started`
    (bind _returnvalue (`GameplayStatics.GetActorOfClass` "/Game/FirstPerson/Blueprints/BP_FirstPersonCharacter.BP_FirstPersonCharacter_C"))
    (`Controller.Possess` (`self.GetController`) (`/Game/FirstPerson/Blueprints/BP_FirstPersonCharacter.PlayerPawn` _returnvalue))))

(event `EnhancedInput|/Game/FirstPerson/Input/Actions/IA_ChainDown`
  (params (ActionValue :type Boolean) (ElapsedSeconds :type "Float (double-precision)") (TriggeredSeconds :type "Float (double-precision)") (InputAction :type "InputAction Object Reference" :default "/Game/FirstPerson/Input/Actions/IA_ChainDown.IA_ChainDown"))
  (bind _movingpiece (`/Game/Blueprints/CageEnigma.MovingPiece` (`self.ObjectInteracting`)))
  ;[1 1 1] Move cylindre left
  (:`Triggered`
    (if (<= (.x (`SceneComponent.K2_GetComponentLocation` _movingpiece)) (.x (`SceneComponent.K2_GetComponentLocation` (`/Game/Blueprints/CageEnigma.Placement4` (`self.LimitMove`)))))
      (`SceneComponent.K2_AddLocalOffset` _movingpiece (`self.MoveVector`) false false))))

(event `EnhancedInput|/Game/FirstPerson/Input/Actions/IA_ChainUp`
  (params (ActionValue :type Boolean) (ElapsedSeconds :type "Float (double-precision)") (TriggeredSeconds :type "Float (double-precision)") (InputAction :type "InputAction Object Reference" :default "/Game/FirstPerson/Input/Actions/IA_ChainUp.IA_ChainUp"))
  (bind _movingpiece (`/Game/Blueprints/CageEnigma.MovingPiece` (`self.ObjectInteracting`)))
  ;[1 1 1] Move cylindre right
  (:`Triggered`
    (if (>= (.x (`SceneComponent.K2_GetComponentLocation` _movingpiece)) (.x (`SceneComponent.K2_GetComponentLocation` (`/Game/Blueprints/CageEnigma.Placement1` (`self.LimitMove`)))))
      (`SceneComponent.K2_AddLocalOffset` _movingpiece (* (`self.MoveVector`) (-1.0 0.0 0.0)) false false))))

(event `self.ResolveCollider.OnComponentBeginOverlap`
  (params (OverlappedComponent :type "PrimitiveComponent Object Reference") (OtherActor :type "Actor Object Reference") (OtherComp :type "PrimitiveComponent Object Reference") (OtherBodyIndex :type Integer) (bFromSweep :type Boolean) (SweepResult :type "HitResult Structure (by ref)"))
  (`KismetSystemLibrary.PrintText` "Enigma resolvesd")
  (`self.PuzzleSolved`))

(event `self.ResolveCollider.OnComponentEndOverlap`
  (params (OverlappedComponent :type "PrimitiveComponent Object Reference") (OtherActor :type "Actor Object Reference") (OtherComp :type "PrimitiveComponent Object Reference") (OtherBodyIndex :type Integer))
  (`KismetSystemLibrary.PrintText` "Enigma unresolvesd")
  (`self.PuzzleUnsolved`))

(fn `UserConstructionScript`)