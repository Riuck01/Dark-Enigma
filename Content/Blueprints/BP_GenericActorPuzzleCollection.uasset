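; BP_GenericActorPuzzleCollection is a puzzle actor that groups child puzzles and counts as solved once all of them are solved.
; SinglePuzzleSovled records a solved child if it belongs to CollectedPuzzles, then compares both list sizes, printing progress or triggering AllPuzzlesSolved.
; AllPuzzlesSolved prints a completion message and calls PuzzleSolved, so collections can nest inside other collections.
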(event `self.ReceiveBeginPlay`
  (`parent.ReceiveBeginPlay`))

(event `SinglePuzzleSovled`
  (params (ARG_SolvedChild :type "/Game/Blueprints/BP_GenericActorPuzzle Object Reference"))
  (bind _collectedpuzzles (`self.CollectedPuzzles`))
  (bind _solvedpuzzles (`self.SolvedPuzzles`))
  (bind _returnvalue (`BlueprintSetLibrary.Set_Length` _solvedpuzzles))
  (bind _returnvalue_2 (`BlueprintSetLibrary.Set_Length` _collectedpuzzles))
  ;[1 1 1] Adds the solved Puzzle is it is part of the Puzzle Collection
  (if (`BlueprintSetLibrary.Set_Contains` _collectedpuzzles ARG_SolvedChild)
    (`BlueprintSetLibrary.Set_Add` _solvedpuzzles ARG_SolvedChild)
    ;[1 1 1] Checks if all Puzzles are solved
    (if (== _returnvalue_2 _returnvalue)
      (`self.AllPuzzlesSolved`)
      (else
        (`KismetSystemLibrary.PrintString` (`KismetStringLibrary.Concat_StrStr` (`KismetStringLibrary.Conv_IntToString` _returnvalue) " of " (`KismetStringLibrary.Conv_IntToString` _returnvalue_2) " puzzles are solved !"))))))

(event `AllPuzzlesSolved`
  (`KismetSystemLibrary.PrintString` "All Puzzles were solved !")
  (`self.PuzzleSolved`) ; Exists just in case this Puzzle Collection is a part of another Puzzle Collection.
)

(fn `UserConstructionScript`)